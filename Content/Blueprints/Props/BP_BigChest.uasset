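; Large loot chest prop that bursts into item pickups when opened, with an item count scaled by the maze generator level.
; Hovering shows a clickable "Chest" world widget, which opens the chest once if a "P"-tagged component is within its sphere.
; Opening removes the widget, plays a sound and rotates the lid by timeline.
; It then spawns a default BP_Item plus random-row ones, registering all with MazeGen for cleanup.
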(event OnComponentEndOverlap(Sphere)
  (params (OverlappedComponent :type Primitive%20Component%20Object%20Reference) (OtherActor :type Actor%20Object%20Reference) (OtherComp :type Primitive%20Component%20Object%20Reference) (OtherBodyIndex :type Integer))
  (if (Components|ComponentHasTag OtherComp "P")
    (Variables|Default|SetAble%20To%20Open false)))

(event OnComponentBeginOverlap(Sphere)
  (params (OverlappedComponent :type Primitive%20Component%20Object%20Reference) (OtherActor :type Actor%20Object%20Reference) (OtherComp :type Primitive%20Component%20Object%20Reference) (OtherBodyIndex :type Integer) (bFromSweep :type Boolean) (SweepResult :type Hit%20Result%20Structure%20%28by%20ref%29))
  (if (Components|ComponentHasTag OtherComp "P")
    (Variables|Default|SetAble%20To%20Open true)))

(event Custom|Bind%20WG%20Button
  (EventDispatchers|BindEventtoOnClicked (Variables|/Game/UI/WG_ItemWorld.WG_ItemWorld_C|GetItemButton (.AsWG%20Item%20World (Utilities|Casting|CastToWG_ItemWorld (UserInterface|GetWidget (Variables|Default|GetWidget))))) (delegate EventInteract)))

(event EventBeginPlay
  (Variables|Default|SetMax%20Number%20Of%20Items (Math|Random|RandomIntegerinRange 3 (+ (Variables|/Game/Blueprints/BP_MazeGen.BP_MazeGen_C|GetGenerator%20Level (Variables|Default|GetMaze%20Gen)) 3)))
  (Default|SetText (.AsWG%20Item%20World (Utilities|Casting|CastToWG_ItemWorld (UserInterface|GetWidget (Variables|Default|GetWidget)))) "Chest")
  (CallFunction|BindWGButton))

(event Collision|EventActorBeginOverlap
  (params (OtherActor :type Actor%20Object%20Reference)))

(event EventTick
  (params (DeltaSeconds :type Float%20%28single-precision%29)))

(event EventEndHover
  (if (not (Game|Player|IsInputKeyDown (Game|GetPlayerController 0) "LeftAlt"))
    (CallFunction|WidgetVisibility false)))

(event EventStartHover
  (CallFunction|WidgetVisibility true))

(event EventInteract
  (bind _returnvalue (Transformation|GetActorLocation))
  (bind _widget (Variables|Default|GetWidget))
  (bind _maze_gen (Variables|Default|GetMaze%20Gen))
  (bind _actors_to_destroy (Variables|/Game/Blueprints/BP_MazeGen.BP_MazeGen_C|GetActors%20To%20Destroy _maze_gen))
  (if (and (Variables|Default|GetAble%20To%20Open) (not (Variables|Default|GetInteracting)))
    (Variables|Default|SetInteracting true)
    (Audio|PlaySound2D "/Game/Sounds/Chest/391947__ssierra1202__chest-openning-crack_Cue.391947__ssierra1202__chest-openning-crack_Cue" 1.0 1.0 0.0 0 0)
    (Development|SetHiddeninGame _widget true false)
    (Components|DestroyComponent _widget)
    (bind _newtrack_0 (Timeline|Timeline PlayFromStart)
      (:Update
        (Transformation|SetRelativeRotation (Variables|Default|GetStaticMesh1) (Math|Rotator|Lerp(Rotator) "0.000000,0.000000,90.000000" "0.000000,0.000000,-20.000000" _newtrack_0 true) false false))
      (:Finished
        (bind _returnvalue_2 (Game|SpawnActorfromClass "/Game/Blueprints/Items/BP_Item.BP_Item_C" (Math|Transform|MakeTransform _returnvalue "0, 0, 0" "1.000000,1.000000,1.000000") "Undefined" "MultiplyWithRoot" 0 "I6" 0))
        (Utilities|Array|Add _actors_to_destroy _returnvalue_2)
        (for _index (range 1 (Variables|Default|GetMax%20Number%20Of%20Items))
          (bind _returnvalue_3 (Game|SpawnActorfromClass "/Game/Blueprints/Items/BP_Item.BP_Item_C" (Math|Transform|MakeTransform _returnvalue "0, 0, 0" "1.000000,1.000000,1.000000") "Undefined" "MultiplyWithRoot" 0 (Utilities|String|StringToName (Utilities|String|Append "I" (Utilities|String|ToString(Integer) (Math|Random|RandomIntegerinRange 1 5)))) 0))
          (Utilities|Array|Add _actors_to_destroy _returnvalue_3))))))

(fn ConstructionScript)

(fn WidgetVisibility
  (params (Visibility :type Boolean))
  (bind _widget (Variables|Default|GetWidget))
  (Utilities|IsValid _widget
    (:Is%20Valid
      (Rendering|SetVisibility _widget Visibility false)
      (bind _output_get (Variables|/Script/Engine.PrimitiveComponent|SetbGenerateOverlapEvents _widget Visibility))
      (Collision|SetCollisionEnabled _widget (select _output_get "QueryOnly" "NoCollision")))))