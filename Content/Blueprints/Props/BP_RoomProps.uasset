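; BP_RoomProps dresses a room at BeginPlay, using its Direction map to count open sides and collect walls.
; It puts the torch on a random wall, or removes it if none exist.
; The open count selects a randomly rotated central prop, random wall-aligned props, or physics crates.
; Wall-prop layouts have a 30% chance to spawn an all-open copy of itself for central crates, with destruction cleanup bound.
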(event Custom|On%20Room%20Destroy
  (params (DestroyedActor :type Actor%20Object%20Reference))
  (Actor|DestroyActor (stale EventBeginPlay _returnvalue)))

(event EventBeginPlay
  (bind _staticmesha (Variables|Default|GetStaticMeshA))
  (bind _walls (Variables|Default|GetWalls))
  (bind _values (Utilities|Map|Values (Variables|Default|GetDirection)))
  (for (_array_element _array_index) _values
    (if _array_element
      (Variables|Default|SetNumber%20Of%20empty (+ (Variables|Default|GetNumber%20Of%20empty) 1))
      (else
        (Utilities|Array|Add (Variables|Default|GetWalls) _array_index))))
  (Utilities|FlowControl|Sequence
    (:then_0
      (if (> (Utilities|Array|Length _walls) 0)
        (bind _keys (Utilities|Map|Keys (Variables|Default|GetDirection)))
        (Variables|Default|SetRandom%20Direction (Utilities|Array|Get(acopy) _keys (.OutItem (Utilities|Array|Random _walls))))
        (Transformation|SetRelativeLocation (Variables|Default|GetRoomTorch) (Utilities|Select :Index (Variables|Default|GetRandom%20Direction) :NewEnumerator0 "375.000000,300.000000,250.000000" :NewEnumerator1 "-300.000000,375.000000,250.000000" :NewEnumerator2 "-375.000000,300.000000,250.000000" :NewEnumerator3 "-300.000000,-375.000000,250.000000") false false)
        (Transformation|SetRelativeRotation (Variables|Default|GetRoomTorch) (Utilities|Select :Index (Variables|Default|GetRandom%20Direction) :NewEnumerator0 "0.000000,90.000000,0.000000" :NewEnumerator1 "0.000000,180.000000,0.000000" :NewEnumerator2 "0.000000,-90.000000,0.000000" :NewEnumerator3 "0, 0, 0") false false)
        (else
          (Components|DestroyComponent (Variables|Default|GetRoomTorch)))))
    (:then_1
      (switch int (Variables|Default|GetNumber%20Of%20empty)
        (:1
          (Components|DestroyComponent (Variables|Default|GetStaticMeshB))
          (Components|StaticMesh|SetStaticMesh _staticmesha (Utilities|Select :Index (Math|Random|RandomIntegerinRange 0 5) :Option%200 "/Game/StaticMesh/Combined_16C54737.Combined_16C54737" :Option%201 "/Game/StaticMesh/Combined_85F1C003.Combined_85F1C003" :Option%202 "/Game/StaticMesh/Combined_A8FCB639.Combined_A8FCB639" :Option%203 "/Game/StaticMesh/Combined_16C54737.Combined_16C54737" :Option%204 "/Game/StaticMesh/Combined_16C54737.Combined_16C54737" :Option%205 "/Game/StaticMesh/Combined_85F1C003.Combined_85F1C003"))
          (Transformation|SetRelativeRotation _staticmesha (Math|Rotator|MakeRotator 0.0 0.0 (Math|Random|RandomFloatinRange 0.0 3.6e+02)) false false))
        (:2
          (bind _keys_2 (Utilities|Map|Keys (Variables|Default|GetDirection) :!label _label))
          (for (_array_element_2 _array_index_2) (Variables|Default|GetWalls)
            (Components|StaticMesh|SetStaticMesh (Utilities|Select :Index _array_index_2 :Option%200 (Variables|Default|GetStaticMeshA) :Option%201 (Variables|Default|GetStaticMeshB)) (Utilities|Select :Index (Math|Random|RandomIntegerinRange 0 5) :Option%200 "/Game/StaticMesh/Combined_16C54737.Combined_16C54737" :Option%201 "/Game/StaticMesh/Combined_85F1C003.Combined_85F1C003" :Option%202 "/Game/StaticMesh/Combined_A8FCB639.Combined_A8FCB639" :Option%203 "/Game/StaticMesh/Combined_110F4126.Combined_110F4126" :Option%204 "/Game/StaticMesh/Combined_82013D72.Combined_82013D72" :Option%205 "/Game/StaticMesh/Combined_8E0425AA.Combined_8E0425AA"))
            (Transformation|SetRelativeLocation (Utilities|Select :Index _array_index_2 :Option%200 (Variables|Default|GetStaticMeshA) :Option%201 (Variables|Default|GetStaticMeshB)) (Utilities|Select :Index (Utilities|Array|Get(acopy) _keys_2 _array_element_2) :NewEnumerator0 "350.000000,0.000000,0.000000" :NewEnumerator1 "0.000000,350.000000,0.000000" :NewEnumerator2 "-350.000000,0.000000,0.000000" :NewEnumerator3 "0.000000,-350.000000,0.000000") false false)
            (Transformation|SetRelativeRotation (Utilities|Select :Index _array_index_2 :Option%200 (Variables|Default|GetStaticMeshA) :Option%201 (Variables|Default|GetStaticMeshB)) (Utilities|Select :Index (Utilities|Array|Get(acopy) _keys_2 _array_element_2) :NewEnumerator0 "0.000000,-90.000000,0.000000" :NewEnumerator1 "0, 0, 0" :NewEnumerator2 "0.000000,90.000000,0.000000" :NewEnumerator3 "0.000000,180.000000,0.000000") false false))
          (switch int (Math|Random|RandomIntegerinRange 0 9)
            (:0
              _)
            (:1
              _)
            (:2
              _))
          (bind _returnvalue (Game|SpawnActorfromClass "BP_RoomProps_C" (Math|Transform|MakeTransform (Transformation|GetActorLocation) "0, 0, 0" "1.000000,1.000000,1.000000") "Undefined" "MultiplyWithRoot" 0 (Utilities|Map|MakeMap "NewEnumerator0" true "NewEnumerator1" true "NewEnumerator2" true "NewEnumerator3" true) 0))
          (Game|BindEventtoOnDestroyed (delegate Custom|On%20Room%20Destroy)))
        (:3
          (Components|DestroyComponent (Variables|Default|GetStaticMeshB))
          (goto _label))
        (:4
          (for _array_element_3 (Utilities|Array|MakeArray (Variables|Default|GetStaticMeshA) (Variables|Default|GetStaticMeshB))
            (Components|StaticMesh|SetStaticMesh _array_element_3 "/Game/StaticMesh/PropItems_Square_Crate_Cube_001.PropItems_Square_Crate_Cube_001")
            (Transformation|SetWorldLocation _array_element_3 (Math|Random|RandomPointinBoundingBox (+ (Transformation|GetActorLocation) "0.000000,0.000000,20.000000") "40.000000,40.000000,1.000000") false false)
            (Variables|/Script/Engine.PrimitiveComponent|SetCanCharacterStepUpOn _array_element_3 "ECB_No")
            (Variables|/Script/Engine.ActorComponent|SetComponentTags _array_element_3 (Utilities|Array|MakeArray "PH"))
            (Physics|SetSimulatePhysics _array_element_3 true)))))))

(fn ConstructionScript)