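; Elevator prop that carries play up from one procedurally generated maze to the next, unlocked by consuming inventory item "I6".
; Unlocking spawns a larger or harder BP_MazeGen above, starts the mechanism spinning, animates the four fences and blends the camera to the elevator.
; Tick moves the actor upward at constant speed, then restores the camera, destroys the previous maze and reverses the fence timeline, after which a platform slides out toward Direction.
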(event OnComponentBeginOverlap(Box)
  (params (OverlappedComponent :type Primitive%20Component%20Object%20Reference) (OtherActor :type Actor%20Object%20Reference) (OtherComp :type Primitive%20Component%20Object%20Reference) (OtherBodyIndex :type Integer) (bFromSweep :type Boolean) (SweepResult :type Hit%20Result%20Structure%20%28by%20ref%29))
  (bind _returnvalue (Game|GetGameMode))
  (bind _childactor (Variables|Default|GetChildActor))
  (bind _generator (Variables|Default|GetGenerator))
  (bind _asbp_top_down_game_mode (Utilities|Casting|CastToBP_TopDownGameMode _returnvalue))
  (bind _childactor_2 (Variables|/Script/Engine.ChildActorComponent|GetChildActor _childactor))
  (bind _max_tiles (Variables|/Game/Blueprints/BP_MazeGen.BP_MazeGen_C|GetMax%20Tiles _generator))
  (bind _generator_level (Variables|/Game/Blueprints/BP_MazeGen.BP_MazeGen_C|GetGenerator%20Level _generator))
  (bind _maze_size (Variables|/Game/Blueprints/BP_MazeGen.BP_MazeGen_C|GetMaze%20Size _generator))
  (bind _returnvalue_2 (+ _generator_level 3))
  (bind _inventory (Variables|/Game/TopDown/Blueprints/BP_TopDownGameMode.BP_TopDownGameMode_C|GetInventory _asbp_top_down_game_mode))
  (bind _returnvalue_3 (Math|Random|RandomIntegerinRange 1 _returnvalue_2))
  (bind _returnvalue_4 (+ _max_tiles _returnvalue_3))
  (if (Components|ComponentHasTag OtherComp "P")
    (if (.ReturnValue (Utilities|Map|Find _inventory "I6"))
      (Utilities|FlowControl|DoOnce false
        (:Completed
          (Collision|SetCollisionEnabled (Variables|Default|GetBox) "NoCollision")
          (Transformation|DetachFromActor _childactor_2 "KeepWorld" "KeepWorld" "KeepWorld")
          (Variables|/Script/Engine.RotatingMovementComponent|SetRotationRate (Variables|/Game/Blueprints/Props/BP_elevatorMechanism.BP_elevatorMechanism_C|GetRotatingMovement (.AsBP%20Elevator%20Mechanism (Utilities|Casting|CastToBP_elevatorMechanism _childactor_2))) "-60.000000,0.000000,0.000000")
          (Utilities|Map|Remove _inventory "I6")
          (Default|Updateinventory (Variables|/Game/TopDown/Blueprints/BP_TopDownGameMode.BP_TopDownGameMode_C|GetWG_Gameplay _asbp_top_down_game_mode) _inventory)
          (Audio|PlaySound2D "/Game/Sounds/Elevator/SC_ElevatorUnlock.SC_ElevatorUnlock" 1.0 1.0 0.0 0 0)
          (bind _output_get (Variables|Default|SetNew%20Center (+ (Transformation|GetActorLocation) "0.000000,0.000000,2500.000000")))
          (Game|SpawnActorfromClass "/Game/Blueprints/BP_MazeGen.BP_MazeGen_C" (Math|Transform|MakeTransform _output_get "0, 0, 0" "1.000000,1.000000,1.000000") "Undefined" "MultiplyWithRoot" 0 true _returnvalue_4 800 (Math|Integer|SelectInt _maze_size (+ _maze_size 1) (< _returnvalue_4 (* _maze_size _maze_size))) (+ (Variables|/Game/Blueprints/BP_MazeGen.BP_MazeGen_C|GetGenerator%20Level _generator) 1) self 0)
          (Utilities|FlowControl|Sequence
            (:then_0
              (Game|Player|SetViewTargetwithBlend (Game|GetPlayerController 0) self 3.0 "VTBlend_Linear" 52.0 true))
            (:then_1
              (CallFunction|StartAnimations)
              (Utilities|FlowControl|Delay 2.0)
              (Variables|Default|SetTick%20Condition true)
              (bind _returnvalue_5 (Audio|CreateSound2D "/Game/Sounds/Elevator/Elevator_Machine_Cue.Elevator_Machine_Cue" 1.0 1.0 0.0 0))
              (bind _output_get_2 (Variables|Default|SetElevator%20Sound _returnvalue_5))
              (Audio|Components|Audio|Play _output_get_2 0.0)))))
      (else
        (Audio|PlaySound2D "/Game/Sounds/Elevator/S_ElevatorFail_Cue.S_ElevatorFail_Cue" 1.0 1.0 0.0 0 0)))))

(event Custom|Start%20Animations
  (bind _platform_relative_location (Variables|Default|GetPlatform%20Relative%20Location))
  (bind (_direction _newtrack_0) (Timeline|Timeline Play)
    (:Update
      (for _array_element (Utilities|Array|MakeArray (Variables|Default|GetFence1) (Variables|Default|GetFence2) (Variables|Default|GetFence3) (Variables|Default|GetFence4))
        (Transformation|SetRelativeLocation _array_element (Math|Vector|MakeVector (.x (Variables|/Script/Engine.SceneComponent|GetRelativeLocation _array_element)) (.y (Variables|/Script/Engine.SceneComponent|GetRelativeLocation _array_element)) (Math|Float|Lerp (Variables|Default|GetOriginal%20fence%20Z) 0.0 _newtrack_0)) false false)))
    (:Finished
      (switch Utilities|FlowControl|Switch|SwitchonETimelineDirection _direction
        (:Backward
          (bind _newtrack_0_2 (Timeline|Timeline_0 Play)
            (:Update
              (Transformation|SetRelativeLocation (Variables|Default|GetElevator_Plane_007) (Math|Vector|Lerp(Vector) _platform_relative_location (Utilities|Select :Index (Variables|Default|GetDirection) :NewEnumerator0 (+ _platform_relative_location "300.000000,0.000000,0.000000") :NewEnumerator1 (+ _platform_relative_location "0.000000,300.000000,0.000000") :NewEnumerator2 (+ _platform_relative_location "-300.000000,0.000000,0.000000") :NewEnumerator3 (+ _platform_relative_location "0.000000,-300.000000,0.000000")) _newtrack_0_2) false false))))))))

(event Custom|fence%20down
  (bind _elevator_sound (Variables|Default|GetElevator%20Sound))
  (bind _platform_relative_location (Variables|Default|GetPlatform%20Relative%20Location))
  (Audio|Components|Audio|Stop _elevator_sound)
  (Audio|Components|Audio|SetSound _elevator_sound "/Game/Sounds/Elevator/Elevator_End_Cue.Elevator_End_Cue")
  (Audio|Components|Audio|Play _elevator_sound 0.0)
  (bind (_direction _newtrack_0) (Timeline|Timeline ReverseFromEnd)
    (:Update
      (for _array_element (Utilities|Array|MakeArray (Variables|Default|GetFence1) (Variables|Default|GetFence2) (Variables|Default|GetFence3) (Variables|Default|GetFence4))
        (Transformation|SetRelativeLocation _array_element (Math|Vector|MakeVector (.x (Variables|/Script/Engine.SceneComponent|GetRelativeLocation _array_element)) (.y (Variables|/Script/Engine.SceneComponent|GetRelativeLocation _array_element)) (Math|Float|Lerp (Variables|Default|GetOriginal%20fence%20Z) 0.0 _newtrack_0)) false false)))
    (:Finished
      (switch Utilities|FlowControl|Switch|SwitchonETimelineDirection _direction
        (:Backward
          (bind _newtrack_0_2 (Timeline|Timeline_0 Play)
            (:Update
              (Transformation|SetRelativeLocation (Variables|Default|GetElevator_Plane_007) (Math|Vector|Lerp(Vector) _platform_relative_location (Utilities|Select :Index (Variables|Default|GetDirection) :NewEnumerator0 (+ _platform_relative_location "300.000000,0.000000,0.000000") :NewEnumerator1 (+ _platform_relative_location "0.000000,300.000000,0.000000") :NewEnumerator2 (+ _platform_relative_location "-300.000000,0.000000,0.000000") :NewEnumerator3 (+ _platform_relative_location "0.000000,-300.000000,0.000000")) _newtrack_0_2) false false))))))))

(event EventBeginPlay
  (Variables|Default|SetOriginal%20fence%20Z (.z (Variables|/Script/Engine.SceneComponent|GetRelativeLocation (Variables|Default|GetFence1))))
  (bind _output_get (Variables|Default|SetOriginal%20Actor%20location (Transformation|GetActorLocation)))
  (Variables|Default|SetTarget%20Actor%20Location (+ _output_get "0.000000,0.000000,2900.000000"))
  (Variables|Default|SetPlatform%20Relative%20Location (Variables|/Script/Engine.SceneComponent|GetRelativeLocation (Variables|Default|GetElevator_Plane_007))))

(event EventTick
  (params (DeltaSeconds :type Float%20%28single-precision%29))
  (bind _returnvalue (Game|GetPlayerController 0))
  (if (Variables|Default|GetTick%20Condition)
    (Transformation|SetActorLocation (Math|Interpolation|VInterptoConstant (Transformation|GetActorLocation) (Math|Vector|Lerp(Vector) (Variables|Default|GetOriginal%20Actor%20location) (Variables|Default|GetTarget%20Actor%20Location) (Variables|Default|GetMax%20Alpha)) DeltaSeconds 3.5e+02) false false)
    (if (Utilities|Operators|EqualEqual (Variables|Default|GetTarget%20Actor%20Location) (Transformation|GetActorLocation) 1e+01)
      (Variables|Default|SetTick%20Condition false)
      (Game|Player|SetViewTargetwithBlend _returnvalue (Pawn|GetControlledPawn _returnvalue) 3.0 "VTBlend_Linear" 52.0 false)
      (Default|DestroyPrevMaze (Variables|Default|GetGenerator))
      (CallFunction|FenceDown))))

(fn ConstructionScript)