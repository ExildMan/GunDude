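; Melee ability hit actor that knocks back tagged actors and scatters tagged components touched by its sphere.
; On BeginPlay it rotates to match the player pawn's forward direction.
; On sphere overlap, actors tagged "E" get a knockback message along that facing.
; Components tagged "PH" receive a random sideways and upward velocity-change impulse, independent of the facing.
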(event OnComponentBeginOverlap(Sphere)
  (params (OverlappedComponent :type Primitive%20Component%20Object%20Reference) (OtherActor :type Actor%20Object%20Reference) (OtherComp :type Primitive%20Component%20Object%20Reference) (OtherBodyIndex :type Integer) (bFromSweep :type Boolean) (SweepResult :type Hit%20Result%20Structure%20%28by%20ref%29))
  (bind _returnvalue (Math|Random|RandomFloatinRange -2.6e+02 -2.2e+02))
  (bind _returnvalue_2 (Math|Random|RandomFloatinRange 2.2e+02 2.6e+02))
  (bind _returnvalue_3 (Math|Random|RandomBool))
  (bind _returnvalue_4 (Math|Float|SelectFloat _returnvalue _returnvalue_2 _returnvalue_3))
  (Utilities|FlowControl|Sequence
    (:then_0
      (if (Actor|ActorHasTag OtherActor "E")
        (Class|BIAI|Knockback(Message) OtherActor (Transformation|GetActorForwardVector))))
    (:then_1
      (if (Components|ComponentHasTag OtherComp "PH")
        (Utilities|IsValid OtherComp
          (:Is%20Valid
            (Physics|AddImpulse OtherComp (Math|Vector|MakeVector _returnvalue_4 _returnvalue_4 (Math|Random|RandomFloatinRange 2e+02 3e+02)) "None" true)))))))

(event EventBeginPlay
  (bind _returnvalue (Game|Player|GetPlayerPawn 0))
  (bind _returnvalue_2 (Transformation|GetActorLocation _returnvalue))
  (Transformation|SetActorRotation (Math|Rotator|FindLookatRotation _returnvalue_2 (+ _returnvalue_2 (Transformation|GetActorForwardVector _returnvalue)))))

(event Collision|EventActorBeginOverlap
  (params (OtherActor :type Actor%20Object%20Reference)))

(event EventTick
  (params (DeltaSeconds :type Float%20%28single-precision%29)))

(fn ConstructionScript)