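; BP_Item is a world loot pickup that takes its data and mesh from a DT_Items row and shows a clickable name widget.
; On spawn it sphere-traces random nearby points for an "F"-tagged landing spot, with capped retries, then scales up while arcing there.
; The widget appears on hover or via the controller's item toggle.
; Interacting within the overlap sphere adds it to the GameMode inventory and destroys it, or bounces it on failure.
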(event OnComponentEndOverlap(Sphere)
  (params (OverlappedComponent :type Primitive%20Component%20Object%20Reference) (OtherActor :type Actor%20Object%20Reference) (OtherComp :type Primitive%20Component%20Object%20Reference) (OtherBodyIndex :type Integer))
  (if (Components|ComponentHasTag OtherComp "P")
    (Variables|Default|SetAble%20To%20Pick false)))

(event OnComponentBeginOverlap(Sphere)
  (params (OverlappedComponent :type Primitive%20Component%20Object%20Reference) (OtherActor :type Actor%20Object%20Reference) (OtherComp :type Primitive%20Component%20Object%20Reference) (OtherBodyIndex :type Integer) (bFromSweep :type Boolean) (SweepResult :type Hit%20Result%20Structure%20%28by%20ref%29))
  (if (Components|ComponentHasTag OtherComp "P")
    (Variables|Default|SetAble%20To%20Pick true)))

(event Custom|Animate%20Item
  (Development|SetHiddeninGame (Variables|Default|GetItem%20Mesh) false false)
  (Variables|Default|SetOriginal%20Actor%20Location (Transformation|GetActorLocation))
  (bind (_direction _movement_alpha _newtrack_1) (Timeline|Timeline PlayFromStart)
    (:Update
      (Transformation|SetWorldScale3D (Variables|Default|GetItem%20Mesh) (Math|Vector|Lerp(Vector) "0, 0, 0" "1.000000,1.000000,1.000000" _newtrack_1))
      (Transformation|SetActorLocation (Math|Vector|Lerp(Vector) (select (< _movement_alpha 0.5) (Variables|Default|GetOriginal%20Actor%20Location) (Variables|Default|GetTarget%20Location)) (+ (Variables|Default|GetOriginal%20Actor%20Location) "0.000000,0.000000,200.000000") _movement_alpha) false true))
    (:Finished
      (Transformation|SetActorLocation (Variables|Default|GetTarget%20Location) false true))))

(event Custom|Show%20Widget
  (Default|SetText (.AsWG%20Item%20World (Utilities|Casting|CastToWG_ItemWorld (UserInterface|GetWidget (Variables|Default|GetWidget)))) (Utilities|Text|ToText(String) (.ItemName (Utilities|Struct|BreakST_Items (Variables|Default|GetItem%20Data)))))
  (EventDispatchers|BindEventtoToggleItems (.AsBP%20Top%20Down%20Controller (Utilities|Casting|CastToBP_TopDownController (Game|GetPlayerController 0))) (delegate Custom|Show%20Items%20Bind)))

(event Custom|Show%20Items%20Bind
  (params (Items%20Visibility :type Boolean) (Alt%20Pressed :type Boolean))
  (CallFunction|WidgetVisibility Items%20Visibility)
  (Variables|Default|SetAlt%20Pressed Alt%20Pressed))

(event EventBeginPlay
  (bind _returnvalue (Transformation|GetActorLocation))
  (while (Utilities|Operators|EqualEqual :A (Variables|Default|GetTarget%20Location))
    (Variables|Default|SetTrys (+ (Variables|Default|GetTrys) 1))
    (bind _outhit (Collision|SphereTraceByChannel (+ _returnvalue "0.000000,0.000000,200.000000") (+ (Math|Random|RandomPointinBoundingBox _returnvalue "800.000000,800.000000,1.000000") (* (Transformation|GetActorUpVector) -500)) 0.0 "TraceTypeQuery2" false 0 "None"))
    (if (or (Components|ComponentHasTag (.HitComponent (Collision|BreakHitResult _outhit)) "F") (== (Variables|Default|GetTrys) 30))
      (Variables|Default|SetTarget%20Location (.ImpactPoint (Collision|BreakHitResult _outhit)))))
  (Utilities|FlowControl|Sequence
    (:then_0
      (CallFunction|AnimateItem))
    (:then_1
      (CallFunction|ShowWidget))
    (:then_2
      (EventDispatchers|BindEventtoOnClicked (Variables|/Game/UI/WG_ItemWorld.WG_ItemWorld_C|GetItemButton (.AsWG%20Item%20World (Utilities|Casting|CastToWG_ItemWorld (UserInterface|GetWidget (Variables|Default|GetWidget))))) (delegate EventInteract)))))

(event EventEndHover
  (if (not (Game|Player|IsInputKeyDown (Game|GetPlayerController 0) "LeftAlt"))
    (CallFunction|WidgetVisibility false)))

(event EventStartHover
  (CallFunction|WidgetVisibility true))

(event EventInteract
  (bind _target_location (Variables|Default|GetTarget%20Location))
  (if (and (Variables|Default|GetAble%20To%20Pick) (not (Variables|Default|GetInteracting)))
    (Variables|Default|SetInteracting true)
    (bind _picked (Default|AddtoInventory (.AsBP%20Top%20Down%20Game%20Mode (Utilities|Casting|CastToBP_TopDownGameMode (Game|GetGameMode))) (Variables|Default|GetRow%20Name)))
    (if _picked
      (Actor|DestroyActor)
      (else
        (bind _newtrack_0 (Timeline|Timeline_0 PlayFromStart)
          (:Update
            (Transformation|SetActorLocation (Math|Vector|Lerp(Vector) _target_location (+ _target_location "0.000000,0.000000,150.000000") _newtrack_0) false true))
          (:Finished
            (Variables|Default|SetInteracting false)))))))

(fn ConstructionScript
  (bind _returnvalue (Utilities|GetDataTableRow "/Game/Blueprints/Items/DT_Items.DT_Items" (Variables|Default|GetRow%20Name))
    (:then
      (bind _output_get (Variables|Default|SetItem%20Data _returnvalue))
      (Components|StaticMesh|SetStaticMesh (Variables|Default|GetItem%20Mesh) (.Mesh (Utilities|Struct|BreakST_Items _output_get))))))

(fn WidgetVisibility
  (params (Visibility :type Boolean))
  (bind _widget (Variables|Default|GetWidget))
  (Rendering|SetVisibility _widget Visibility false)
  (bind _output_get (Variables|/Script/Engine.PrimitiveComponent|SetbGenerateOverlapEvents _widget Visibility))
  (Collision|SetCollisionEnabled _widget (select _output_get "QueryOnly" "NoCollision")))