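; BP_MazeGen is a maze generator Blueprint that, in this graph, only handles reporting tile loading to the loading screen.
; On BeginPlay it casts the game mode to BP_TopDownGameMode and, unless Continue is set, shows the loading widget and sets its percent once.
; CalcTileLoading derives that value from the CurrentTiles to MaxTiles ratio, scaled to peak at 0.4 when all tiles exist.
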(event EventBeginPlay
  (Variables|Default|SetAs%20BP%20Top%20Down%20Game%20Mode (.AsBP%20Top%20Down%20Game%20Mode (Utilities|Casting|CastToBP_TopDownGameMode (Game|GetGameMode))))
  (if (not (Variables|Default|GetContinue))
    (Default|ShowLoading (Variables|Default|GetAs%20BP%20Top%20Down%20Game%20Mode))
    (Default|SetPercent (Variables|/Game/TopDown/Blueprints/BP_TopDownGameMode.BP_TopDownGameMode_C|GetWG_Loading (Variables|Default|GetAs%20BP%20Top%20Down%20Game%20Mode)) (CallFunction|CalcTileLoading))))

(fn ConstructionScript)

(fn CalcTileLoading
  (return (/ 4e+01 (* (/ (Math|Conversions|ToFloat(Integer) (Variables|Default|GetMax%20Tiles)) (Math|Conversions|ToFloat(Integer) (Variables|Default|GetCurrent%20Tiles))) 1e+02))))