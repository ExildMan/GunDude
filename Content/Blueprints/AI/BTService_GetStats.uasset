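; Behavior tree service that keeps an AI pawn's blackboard in sync with its current stats.
; Each tick it sets the enemy key to the first player pawn if no valid enemy is stored.
; It then calls GetStatsMessage on the controlled pawn and copies the returned death flags, sight and range flags, state and host location into blackboard keys.
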(event EventReceiveTickAI
  (params (OwnerController :type AI%20Controller%20Object%20Reference) (ControlledPawn :type Pawn%20Object%20Reference) (DeltaSeconds :type Float%20%28single-precision%29))
  (bind _bb_enemy (Variables|Default|GetBB%20Enemy))
  (Utilities|FlowControl|Sequence
    (:then_0
      (Utilities|IsValid (AI|BehaviorTree|GetBlackboardValueasActor _bb_enemy)
        (:Is%20Not%20Valid
          (Class|BTFunctionLibrary|SetBlackboardValueasObject _bb_enemy (Game|Player|GetPlayerPawn 0)))))
    (:then_1
      (bind (_dead _hostdead _insight _inrange _state _host_location) (Class|BIAI|GetStats(Message) ControlledPawn))
      (Class|BTFunctionLibrary|SetBlackboardValueasBool (Variables|Default|GetBB%20Dead) _dead)
      (Class|BTFunctionLibrary|SetBlackboardValueasBool (Variables|Default|GetBB%20Host%20Dead) _hostdead)
      (Class|BTFunctionLibrary|SetBlackboardValueasBool (Variables|Default|GetBB%20insight) _insight)
      (Class|BTFunctionLibrary|SetBlackboardValueasBool (Variables|Default|GetBB%20InRange) _inrange)
      (Class|BTFunctionLibrary|SetBlackboardValueasEnum (Variables|Default|GetBB%20STate) _state)
      (AI|BehaviorTree|SetBlackboardValueasVector (Variables|Default|GetBB%20hostLocation) _host_location))))