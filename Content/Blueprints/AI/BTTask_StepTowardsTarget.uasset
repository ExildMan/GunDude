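; Behavior tree task that picks a random reachable move destination near the first player's pawn for the AI.
; It sends MovementRotationMessage to the controlled pawn, then samples navigation around a point offset from the player using cosine and sine of random angles within a half-circle range.
; On success it sets the controller's focal point and the BBMoveTo blackboard key to that location, otherwise the task fails.
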(event EventReceiveExecuteAI
  (params (OwnerController :type AI%20Controller%20Object%20Reference) (ControlledPawn :type Pawn%20Object%20Reference))
  (bind _returnvalue (Math|Trig|GetPI))
  (bind _returnvalue_2 (Game|Player|GetPlayerPawn 0))
  (bind _returnvalue_3 (Transformation|GetActorLocation _returnvalue_2))
  (bind _returnvalue_4 (* _returnvalue 2.0))
  (bind _returnvalue_5 (Math|Random|RandomFloatinRange _returnvalue _returnvalue_4))
  (bind (_x _y _z) (Math|Vector|BreakVector _returnvalue_3))
  (bind _returnvalue_6 (Math|Trig|Cos(Radians) _returnvalue_5))
  (bind _returnvalue_7 (Math|Trig|Sin(Radians) _returnvalue_5))
  (bind _returnvalue_8 (* _returnvalue_7 5e+02))
  (bind _returnvalue_9 (* _returnvalue_6 5e+02))
  (bind _returnvalue_10 (+ _returnvalue_9 _x))
  (bind _returnvalue_11 (+ _returnvalue_8 _y))
  (bind (_randomlocation _returnvalue_12) (AI|Navigation|GetRandomReachablePointinRadius (Math|Vector|MakeVector _returnvalue_10 _returnvalue_11 _z) 2e+02 0 0))
  (Class|BIAI|MovementRotation(Message) ControlledPawn)
  (if _returnvalue_12
    (bind _output_get (Variables|Default|SetRandom%20Location _randomlocation))
    (AI|SetFocalPoint OwnerController _output_get)
    (AI|BehaviorTree|SetBlackboardValueasVector (Variables|Default|GetBB%20MoveTo) _output_get)
    (AI|BehaviorTree|FinishExecute true)
    (else
      (AI|BehaviorTree|FinishExecute false))))