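; Hell Gate enemy structure that spawns AI_Enemy1 zombies around itself on BeginPlay, their count scaled by the generator's level.
; While the player is inside its sphere, it swaps sigil materials and a looping timer fires bullets when a line trace confirms sight.
; Damage shrinks the rotating mesh with remaining health; death explodes it, resets the tile floor material and flags its zombies as host-dead.
; A timeline pulses its red light.
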(event OnComponentBeginOverlap(Sphere)
  (params (OverlappedComponent :type Primitive%20Component%20Object%20Reference) (OtherActor :type Actor%20Object%20Reference) (OtherComp :type Primitive%20Component%20Object%20Reference) (OtherBodyIndex :type Integer) (bFromSweep :type Boolean) (SweepResult :type Hit%20Result%20Structure%20%28by%20ref%29))
  (if (Components|ComponentHasTag OtherComp "P")
    (Variables|Default|SetFire true)
    (Rendering|Material|SetMaterial (Variables|Default|GetStaticMesh) 0 "/Game/Materials/SigilMM_Inst3.SigilMM_Inst3")
    (Default|PlayActionMusic (.AsBP%20Top%20Down%20Character (Utilities|Casting|CastToBP_TopDownCharacter OtherActor)))))

(event OnComponentEndOverlap(Sphere)
  (params (OverlappedComponent :type Primitive%20Component%20Object%20Reference) (OtherActor :type Actor%20Object%20Reference) (OtherComp :type Primitive%20Component%20Object%20Reference) (OtherBodyIndex :type Integer))
  (if (Components|ComponentHasTag OtherComp "P")
    (Variables|Default|SetFire false)
    (Rendering|Material|SetMaterial (Variables|Default|GetStaticMesh) 0 "/Game/Materials/SigilMM.SigilMM")))

(event Custom|Death
  (Effects|SpawnEmitteratLocation "/Game/Particles/P_Explosion.P_Explosion" (Transformation|GetActorLocation) "0, 0, 0" "5.000000,5.000000,5.000000")
  (Rendering|Material|SetMaterial (Variables|/Game/Blueprints/BP_Tile.BP_Tile_C|GetFloor (Variables|Default|GetTile)) 0 "/Game/Materials/Empty.Empty")
  (for _array_element (Variables|Default|GetMy%20Zombies)
    (Variables|/Game/Blueprints/AI/AI_Enemy1.AI_Enemy1_C|SetHostDead _array_element true))
  (Actor|DestroyActor))

(event Custom|Shooty
  (if (Variables|Default|GetFire)
    (bind (_outhit _returnvalue) (Collision|LineTraceByChannel (Transformation|GetWorldLocation (Variables|Default|GetStaticMesh1)) (Transformation|GetActorLocation (Game|Player|GetPlayerPawn 0)) "TraceTypeQuery2" false 0 "None"))
    (if _returnvalue
      (if (Components|ComponentHasTag (.HitComponent (Collision|BreakHitResult _outhit)) "P")
        (Game|SpawnActorfromClass "/Game/Blueprints/Abilities/BP_HellGateBullet.BP_HellGateBullet_C" (Math|Transform|MakeTransform (Transformation|GetWorldLocation (Variables|Default|GetStaticMesh1)) "0, 0, 0" "1.000000,1.000000,1.000000") "Undefined" "MultiplyWithRoot" 0 0)
        (Audio|PlaySound2D "/Engine/VREditor/Sounds/UI/Dockable_Window_Close.Dockable_Window_Close" 1.0 1.0 0.0 0 0)))))

(event EventBeginPlay
  (bind _returnvalue (Transformation|GetActorLocation))
  (bind _pointlight (Variables|Default|GetPointLight))
  (bind _generator (Variables|Default|GetGenerator))
  (bind _generator_level (Variables|/Game/Blueprints/BP_MazeGen.BP_MazeGen_C|GetGenerator%20Level _generator))
  (Components|Movement|SetUpdatedComponent (Variables|Default|GetRotatingMovement) (Variables|Default|GetStaticMesh1))
  (Variables|Default|SetCurrent%20Health (Variables|Default|GetMax%20Health))
  (Variables|Default|SetOriginal%20Scale (Transformation|GetWorldScale (Variables|Default|GetStaticMesh1)))
  (Utilities|FlowControl|Sequence
    (:then_0
      (bind _light_alpha (Timeline|Timeline PlayFromStart)
        (:Update
          (Rendering|Components|Light|SetLightColor _pointlight (Math|Color|Lerp(LinearColor) "(R=0.474510,G=0.003922,B=0.050980,A=1.000000)" "(R=1.000000,G=0.017360,B=0.000000,A=1.000000)" _light_alpha) true)
          (Rendering|Components|Light|SetIntensity _pointlight (Math|Float|Lerp 1.5e+02 1.8e+02 _light_alpha))
          (Rendering|Lighting|SetAttenuationRadius _pointlight (Math|Float|Lerp 7e+02 8e+02 _light_alpha)))))
    (:then_1
      (Utilities|Time|SetTimerbyEvent (delegate Custom|Shooty) 0.3 true))
    (:then_2
      (for _index (range 0 (- (Math|Random|RandomIntegerinRange _generator_level (Math|Integer|SelectInt (+ _generator_level 1) _generator_level (Math|Random|RandomBool))) 1))
        (bind _returnvalue_2 (Game|SpawnActorfromClass "/Game/Blueprints/AI/AI_Enemy1.AI_Enemy1_C" (Math|Transform|MakeTransform (Math|Random|RandomPointinBoundingBox (+ _returnvalue "0.000000,0.000000,40.000000") "300.000000,300.000000,1.000000") "0, 0, 0" "1.000000,1.000000,1.000000") "Undefined" "MultiplyWithRoot" 0 (Variables|Default|GetGenerator) _returnvalue 0))
        (Utilities|Array|Add (Variables|/Game/Blueprints/BP_MazeGen.BP_MazeGen_C|GetActors%20To%20Destroy (Variables|Default|GetGenerator)) _returnvalue_2)
        (Utilities|Array|Add (Variables|Default|GetMy%20Zombies) _returnvalue_2)))))

(event Collision|EventActorBeginOverlap
  (params (OtherActor :type Actor%20Object%20Reference)))

(event EventTick
  (params (DeltaSeconds :type Float%20%28single-precision%29)))

(event Game|Damage|EventAnyDamage
  (params (Damage :type Float%20%28single-precision%29) (DamageType :type Damage%20Type%20Object%20Reference) (InstigatedBy :type Controller%20Object%20Reference) (DamageCauser :type Actor%20Object%20Reference))
  (bind _original_scale (Variables|Default|GetOriginal%20Scale))
  (bind _output_get (Variables|Default|SetCurrent%20Health (Math|Float|Clamp(Float) (- (Variables|Default|GetCurrent%20Health) Damage) 0.0 (Variables|Default|GetMax%20Health))))
  (if (<= _output_get 0.0)
    (CallFunction|Death)
    (else
      (Transformation|SetWorldScale3D (Variables|Default|GetStaticMesh1) (Math|Vector|Lerp(Vector) (/ _original_scale 5) _original_scale (/ (Variables|Default|GetCurrent%20Health) (Variables|Default|GetMax%20Health)))))))

(fn ConstructionScript)