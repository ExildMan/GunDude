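; BP_TIle is a tile Blueprint that shows its number and marks its open directions with north, east, south and west arrows.
; The Construction Script writes the tile number to a text component, then ToggleArrows sets each arrow's visibility from the Directions map.
; FindExit holds logic to open the incoming side's opposite and pick a random remaining exit, but it is disconnected and never runs.
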(event EventBeginPlay)

(event Collision|EventActorBeginOverlap
  (params (OtherActor :type Actor%20Object%20Reference)))

(event EventTick
  (params (DeltaSeconds :type Float%20%28single-precision%29)))

(fn ConstructionScript
  (Rendering|Components|TextRender|SetText (Variables|Default|GetT_Tile%20Number) (Utilities|Text|ToText(String) (Utilities|String|Append "Tile Number is :" (Utilities|String|ToString(Integer) (Variables|Default|GetTileNumber)))))
  (CallFunction|ToggleArrows))

(fn FindExit
  (params (Income%20Direction :type E_Directions%20Enum :default "NewEnumerator0")))

(fn ToggleArrows
  (bind _keys (Utilities|Map|Keys (Variables|Default|GetDirections)))
  (for _array_element _keys
    (Rendering|SetVisibility (Utilities|Select :Index _array_element :NewEnumerator0 (Variables|Default|GetArrow%20North) :NewEnumerator1 (Variables|Default|GetArrow%20East) :NewEnumerator2 (Variables|Default|GetArrow%20South) :NewEnumerator3 (Variables|Default|GetArrow%20West)) (.Value (Utilities|Map|Find (Variables|Default|GetDirections) _array_element)) true))
  (return))